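; BP_Plane is a player-flown plane that constantly moves forward and fires homing missiles.
; Pitch and Roll axes rotate it locally, scaled by frame time and look or turn speed.
; Fire runs SelectNearTarget over all BP_Target actors, then spawns a BP_Missile at FirePivot homing on the result.
; The nearest-target search seeds its minimum distance from the plane's own location, yielding zero, so the first target found always wins.
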(event `self.ReceiveBeginPlay`)

(event `self.ReceiveTick`
  (params (DeltaSeconds :type "Float (single-precision)"))
  (`self.AddMovementInput` (`self.GetActorForwardVector`)))

(event `InputAxis|Pitch`
  (params (AxisValue :type "Float (single-precision)"))
  (`self.K2_AddActorLocalRotation` (`KismetMathLibrary.MakeRotator` 0.0 (* AxisValue (`GameplayStatics.GetWorldDeltaSeconds`) (`self.LookSpeed`)))))

(event `InputAxis|Roll`
  (params (AxisValue :type "Float (single-precision)"))
  (`self.K2_AddActorLocalRotation` (`KismetMathLibrary.MakeRotator` (* AxisValue (`GameplayStatics.GetWorldDeltaSeconds`) (`self.TurnSpeed`)))))

(event `InputAction|Fire`
  (params (Key :type "Key Structure"))
  (:`Pressed`
    (`self.SelectNearTarget`)
    (`/Engine/EditorBlueprintResources/StandardMacros.IsValid` (`self.Target`)
      (:`Is Valid`
        (`|SpawnActorFromClass` "/Game/Blueprints/BP_Missile.BP_Missile_C" (`SceneComponent.K2_GetComponentToWorld` (`self.FirePivot`)) "Undefined" "MultiplyWithRoot" null (`self.GetComponentByClass` (`self.Target`) "/Script/Engine.SceneComponent") null)))))

(fn `SelectNearTarget`
  (set `self.Target` null)
  (bind _outactors (`GameplayStatics.GetAllActorsOfClass` "/Game/Blueprints/BP_Target.BP_Target_C"))
  (for (_array_element _array_index) _outactors
    (if (== _array_index 0)
      (set `self.MinDistance` (`KismetMathLibrary.VSize` (- (`self.K2_GetActorLocation`) (`self.K2_GetActorLocation`))))
      (set `self.Target` _array_element)
      (else
        (bind _returnvalue (`KismetMathLibrary.VSize` (- (`self.K2_GetActorLocation` _array_element) (`self.K2_GetActorLocation`))))
        (if (< _returnvalue (`self.MinDistance`))
          (set `self.MinDistance` _returnvalue)
          (set `self.Target` _array_element))))))

(fn `UserConstructionScript`)